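; BP_DVDDirt is a dirt decal actor, apparently on a DVD, that is cleaned by wiping with a rag.
; Construction picks a random decal material from Dirts.
; Each Box overlap by a "Rag"-tagged component removes random HP and slightly shrinks the decal, destroying the actor at zero.
; Despite its name, UpdateDecalOpacity only changes scale; the dynamic material created at BeginPlay is never assigned to the decal.
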(event `self.ReceiveBeginPlay`
  (bind _returnvalue (`KismetMaterialLibrary.CreateDynamicMaterialInstance` (`DecalComponent.DecalMaterial` (`self.Decal1`))))
  (bind _output_get (set `self.DVDDecal` _returnvalue))
  (`MaterialInstanceDynamic.SetScalarParameterValue` _output_get "Opacity" 0.01))

(event `self.Box.OnComponentBeginOverlap`
  (params (OverlappedComponent :type "PrimitiveComponent Object Reference") (OtherActor :type "Actor Object Reference") (OtherComp :type "PrimitiveComponent Object Reference") (OtherBodyIndex :type Integer) (bFromSweep :type Boolean) (SweepResult :type "HitResult Structure (by ref)"))
  (if (`ActorComponent.ComponentHasTag` OtherComp "Rag")
    (bind _output_get (set `self.HP` (- (`self.HP`) (`KismetMathLibrary.RandomFloatInRange` 10.0 25.0))))
    (`self.UpdateDecalOpacity` _output_get)
    (if (<= (`self.HP`) 0.0)
      (`KismetSystemLibrary.PrintString` "CLEAN!")
      (`self.K2_DestroyActor`))))

(event `self.ReceiveAnyDamage`
  (params (Damage :type "Float (single-precision)") (DamageType :type "DamageType Object Reference") (InstigatedBy :type "Controller Object Reference") (DamageCauser :type "Actor Object Reference")))

(fn `UpdateDecalOpacity`
  (params (Input :type "Float (double-precision)"))
  (bind _decal1 (`self.Decal1`))
  (bind (_returnvalue_x _returnvalue_y _returnvalue_z) (`KismetMathLibrary.BreakVector` (`SceneComponent.K2_GetComponentScale` _decal1)))
  (`SceneComponent.SetWorldScale3D` _decal1 (`KismetMathLibrary.MakeVector` _returnvalue_x (- _returnvalue_y 0.002) (- _returnvalue_z 0.002))))

(fn `UserConstructionScript`
  (`DecalComponent.SetDecalMaterial` (`self.Decal1`) (`KismetArrayLibrary.Array_Random` (`self.Dirts`))))