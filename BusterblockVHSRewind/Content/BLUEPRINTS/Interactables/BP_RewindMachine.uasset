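; Possessable VHS rewind station where the player inserts a tape and holds a button to rewind it.
; Overlapping tapes leave the player's hand and tween into the holder via the tape's physics handle.
; Rewinding advances tape progress and resizes reels while timers build heat; overheating locks rewinding during a tweened cooldown.
; A looping cursor trace moves a detection component, whose end overlap with the button stops rewinding.
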(event `InitProgress`
  (bind _tape (`self.Tape`))
  (bind _tapeprogress (`/Game/BLUEPRINTS/Interactables/BP_VHSTape.TapeProgress` _tape))
  (bind _asynctaskproxy (`FCTweenBPActionFloat.TweenFloat` 0.0 1.0 0.1 "Linear" 0.0 0.0 0.0 -1)
    (:`then`
      (bind _output_get (set `self.TapeProgressTimer` _asynctaskproxy))
      (`FCTweenBPAction.Pause` _output_get))
    (:`ApplyEasing`
      (if (< _tapeprogress 100.0)
        (bind _output_get_2 (set `/Game/BLUEPRINTS/Interactables/BP_VHSTape.TapeProgress` (+ _tapeprogress 0.2) _tape))
        (`/Game/BLUEPRINTS/Interactables/BP_VHSTape.AdjustTapeSize` _tape _output_get_2 (`/Game/BLUEPRINTS/Interactables/BP_VHSTape.TapeProgressEnd` _tape))
        (if (>= _tapeprogress 100.0)
          (`/Engine/EditorBlueprintResources/StandardMacros.DoOnce` false :!label _label
            (:`Completed`
              ;[0 1 0.1351] Tape is finished
              (`GameplayStatics.PlaySound2D` "/Game/Audio/SND_Tape_Rewind_Finished.SND_Tape_Rewind_Finished" 1.0 1.0 0.0 null null)
              (set `/Game/BLUEPRINTS/Interactables/BP_VHSTape.isRewound?` true _tape)
              (`/Game/BLUEPRINTS/InteractionBPI.StopInteracting`)
              (`KismetSystemLibrary.K2_PauseTimerHandle` (`self.HeatTimer`))
              (`FCTweenBPAction.Pause` (`self.TapeProgressTimer`))
              (`self.StopRewindTape`))))))))

(event `self.ReceiveBeginPlay`
  (`SceneComponent.SetVisibility` (`self.ProgresBarW`) false false)
  (set `self.RewindDefaultLocation` (`SceneComponent.K2_GetComponentLocation` (`self.BP_RewindMachine_Button`)))
  (bind _returnvalue (`GameplayStatics.CreateSound2D` "/Game/Audio/SND_Tape_Rewind_Loop.SND_Tape_Rewind_Loop" 1.0 1.0 0.0 null))
  (set `self.RewindLoop` _returnvalue)
  (set `self.TapeROT` (`SceneComponent.K2_GetComponentRotation` (`self.TapeHolder`)))
  (bind _returnvalue_2 (`KismetSystemLibrary.K2_SetTimer` null "HeatCooldown" 0.5 true))
  (bind _output_get (set `self.heatCooldownTimer` _returnvalue_2))
  (`KismetSystemLibrary.K2_PauseTimerHandle` _output_get)
  (add `AudioComponent.OnAudioPlaybackPercent` (`self.RewindLoop`) (delegate `OnAudioPlaybackPercentEvent`)))

(event `OnAudioPlaybackPercentEvent`
  (params (PlayingSoundWave :type "SoundWave Object Reference") (PlaybackPercent :type "Float (single-precision)"))
  (set `self.CurrentRewindLoopPosition` (* PlaybackPercent (`SoundBase.Duration` PlayingSoundWave))))

(event `self.ReceiveTick`
  (params (DeltaSeconds :type "Float (single-precision)")))

(event `ResetFullTape`
  (goto _label :!via `Reset`))

(event `/Game/BLUEPRINTS/PossessStationBPI.PossessStation`
  (bind _returnvalue (`GameplayStatics.GetPlayerController` 0))
  ;[0 1 0.1351] When possessed
  (`PlayerController.SetViewTargetWithBlend` (`GameplayStatics.GetPlayerController` 0) self 0.5 "VTBlend_EaseInOut" 10.0 true)
  (`KismetSystemLibrary.Delay` 0.5)
  (`PrimitiveComponent.SetCollisionEnabled` (`self.SM_RewindMachine`) "NoCollision")
  (`Controller.Possess` _returnvalue self)
  (`self.EnableInput` _returnvalue)
  (`self.Tape`
    (:`then`
      (`SceneComponent.SetVisibility` (`self.ProgresBarW`) true false)
      (bind _asw_press_to_rewind (cast `/Game/BLUEPRINTS/WIDGETS/W_PressToRewind` (`WidgetComponent.GetUserWidgetObject` (`self.PressRewindButtonW`))))
      (`/Game/BLUEPRINTS/WIDGETS/W_PressToRewind.Start` _asw_press_to_rewind))
    (:`else`)))

(event `InsertTape`
  (bind _tape (`self.Tape`))
  (bind _sm_vhstape (`/Game/BLUEPRINTS/Interactables/BP_VHSTape.SM_VHSTape` _tape))
  ;[0 1 0.1351] Insert Tape into machine animation
  (bind _asw_tape_rewind_progressbar (cast `/Game/BLUEPRINTS/WIDGETS/W_TapeRewind_Progressbar` (`WidgetComponent.GetUserWidgetObject` (`self.ProgresBarW`))))
  (bind _tape_2 (`self.Tape`)
    (:`then`
      (`ActorComponent.Activate` (`/Game/BLUEPRINTS/Interactables/BP_Interactable_Master.PhysicsHandle` _tape_2) true)
      (set `/Game/BLUEPRINTS/WIDGETS/W_TapeRewind_Progressbar.CurrentTape` (`self.Tape`) _asw_tape_rewind_progressbar)
      (set `/Game/BLUEPRINTS/WIDGETS/W_TapeRewind_Progressbar.RewindMachineRef` self _asw_tape_rewind_progressbar)
      (bind _sm_vhstape_2 (`/Game/BLUEPRINTS/Interactables/BP_VHSTape.SM_VHSTape` _tape_2))
      (bind (_asynctaskproxy _value) (`FCTweenBPActionRotator.TweenRotator` (`SceneComponent.K2_GetComponentRotation` _sm_vhstape_2) (struct :`Yaw` -90.0) 0.25 "InOutSine")
        (:`ApplyEasing`
          (`SceneComponent.K2_SetWorldRotation` _sm_vhstape_2 _value false false))
        (:`OnComplete`
          (`PhysicsHandleComponent.ReleaseComponent` (`/Game/BLUEPRINTS/Interactables/BP_Interactable_Master.PhysicsHandle` (`self.Tape`)))
          (`PhysicsHandleComponent.GrabComponentAtLocationWithRotation` :`self` (`/Game/BLUEPRINTS/Interactables/BP_VHSTape.PhysicsHandle` _tape) :`Component` _sm_vhstape :`Location` (`SceneComponent.K2_GetComponentLocation` _sm_vhstape))
          (set `/Game/BLUEPRINTS/Interactables/BP_VHSTape.isInteractable?` false (`self.Tape`))
          (bind _tape_3 (`self.Tape`)
            (:`then`
              (bind _physicshandle (`/Game/BLUEPRINTS/Interactables/BP_Interactable_Master.PhysicsHandle` _tape_3))
              (bind (_asynctaskproxy_2 _value_2) (`FCTweenBPActionVector.TweenVector` (`PhysicsHandleComponent.GetTargetLocationAndRotation` _physicshandle) (`SceneComponent.K2_GetComponentLocation` (`self.TapeHolder`)) 0.25 "InOutSine")
                (:`then`
                  (`KismetSystemLibrary.Delay` 0.1)
                  (bind _sm_vhstape_3 (`/Game/BLUEPRINTS/Interactables/BP_VHSTape.SM_VHSTape` _tape_3))
                  (`/Engine/EditorBlueprintResources/StandardMacros.IsValid` _sm_vhstape_3
                    (:`Is Valid`
                      (`GameplayStatics.PlaySoundAtLocation` "/Game/Audio/SND_Tape_Rewind_Inserted_Cue.SND_Tape_Rewind_Inserted_Cue" (`SceneComponent.K2_GetComponentLocation` _sm_vhstape_3) (struct) 1.0 1.0 0.0 null null null null))))
                (:`ApplyEasing`
                  (`PhysicsHandleComponent.SetTargetLocation` _physicshandle _value_2))
                (:`OnComplete`
                  (set `self.isInteractable?` true)
                  (set `/Game/BLUEPRINTS/Interactables/BP_VHSTape.isInteractable?` true (`self.Tape`))
                  (`PhysicsHandleComponent.ReleaseComponent` (`/Game/BLUEPRINTS/Interactables/BP_Interactable_Master.PhysicsHandle` (`self.Tape`)))
                  (set `self.isBusy?` true))))
            (:`else`)))))
    (:`else`)))

(event `self.TapeDetection.OnComponentEndOverlap`
  (params (OverlappedComponent :type "PrimitiveComponent Object Reference") (OtherActor :type "Actor Object Reference") (OtherComp :type "PrimitiveComponent Object Reference") (OtherBodyIndex :type Integer))
  ;[1 0 0] Exit tray
  (cast `/Game/BLUEPRINTS/Interactables/BP_VHSTape` OtherActor)
  (`self.ResetTapeDetection`))

(event `self.TapeDetection.OnComponentBeginOverlap`
  (params (OverlappedComponent :type "PrimitiveComponent Object Reference") (OtherActor :type "Actor Object Reference") (OtherComp :type "PrimitiveComponent Object Reference") (OtherBodyIndex :type Integer) (bFromSweep :type Boolean) (SweepResult :type "HitResult Structure (by ref)"))
  (bind _tape (`self.Tape`))
  (bind _physicshandle (`/Game/BLUEPRINTS/Interactables/BP_VHSTape.PhysicsHandle` _tape))
  (bind _sm_vhstape (`/Game/BLUEPRINTS/Interactables/BP_VHSTape.SM_VHSTape` _tape))
  (bind _returnvalue (`SceneComponent.K2_GetComponentLocation` _sm_vhstape))
  ;[0 1 0.1351] Insert Tape from Players Hands
  (if (not (`self.isBusy?`))
    (bind _asbp_vhstape (cast `/Game/BLUEPRINTS/Interactables/BP_VHSTape` OtherActor))
    (set `self.Tape` _asbp_vhstape)
    (`/Engine/EditorBlueprintResources/StandardMacros.DoOnce` false :!label _label_2
      (:`Completed`
        (set `self.isBusy?` true)
        (`ActorComponent.SetActive` _physicshandle true true)
        (`PhysicsHandleComponent.GrabComponentAtLocationWithRotation` :`self` _physicshandle :`Component` _sm_vhstape :`Location` _returnvalue)
        (bind (_asynctaskproxy _value) (`FCTweenBPActionVector.TweenVector` _returnvalue (`SceneComponent.K2_GetComponentLocation` (`self.Arrow`)) 0.25 "InOutSine")
          (:`then`
            (`PrimitiveComponent.SetCollisionEnabled` (`self.ClickBox`) "QueryOnly")
            (`SceneComponent.SetVisibility` (`self.PressRewindButtonW`) true false)
            (bind _returnvalue_2 (`GameplayStatics.GetActorOfClass` "/Game/MODELS/FirstPerson/Blueprints/BP_FirstPersonCharacter.BP_FirstPersonCharacter_C"))
            (`/Game/MODELS/FirstPerson/Blueprints/BP_FirstPersonCharacter.ReleaseObjectFromHand` _returnvalue_2))
          (:`ApplyEasing`
            (`PhysicsHandleComponent.SetTargetLocation` _physicshandle _value))
          (:`OnComplete`
            (`/Engine/EditorBlueprintResources/StandardMacros.DoOnce` false :!label _label_3
              (:`Completed`
                (`self.InsertTape`)))))))))

(event `ResetTapeDetection`
  ;[0 1 0.1351] Insert Tape from Players Hands
  (`|ExecutionSequence`
    (:`then_0`
      (goto _label_2 :!via `Reset`))
    (:`then_1`
      (goto _label_3 :!via `Reset`))))

(event `self.Tray.OnComponentEndOverlap`
  (params (OverlappedComponent :type "PrimitiveComponent Object Reference") (OtherActor :type "Actor Object Reference") (OtherComp :type "PrimitiveComponent Object Reference") (OtherBodyIndex :type Integer))
  ;[1 0 0] Exit tray
  (cast `/Game/BLUEPRINTS/Interactables/BP_VHSTape` OtherActor)
  (`self.ResetTapeDetection`)
  (`/Game/BLUEPRINTS/InteractionBPI.StopInteracting`)
  (set `self.Tape` null)
  (set `self.isBusy?` false)
  (`self.ResetFullTape`))

(event `/Game/BLUEPRINTS/PossessStationBPI.ExitedStation`
  ;[0 1 0.1351] Triggered when Exitting or interrupting Session
  (`PrimitiveComponent.SetCollisionEnabled` (`self.SM_RewindMachine`) "QueryAndPhysics")
  (`self.PauseRewind`)
  (`SceneComponent.SetVisibility` (`self.ProgresBarW`) false false)
  (`SceneComponent.SetVisibility` (`self.PressRewindButtonW`) false false)
  (set `self.Tape` null)
  (`PrimitiveComponent.SetCollisionEnabled` (`self.ClickBox`) "NoCollision"))

(event `PauseRewind`
  ;[0 1 0.1351] Pause rewind function
  (`AudioComponent.SetPaused` (`self.RewindLoop`) true)
  (bind _tape (`self.Tape`)
    (:`then`
      (if (< (`/Game/BLUEPRINTS/Interactables/BP_VHSTape.TapeProgress` _tape) 100.0)
        (bind _tapeprogresstimer (`self.TapeProgressTimer`)
          (:`then`
            (`FCTweenBPAction.Pause` _tapeprogresstimer)
            (`KismetSystemLibrary.K2_PauseTimerHandle` (`self.HeatTimer`))
            (`KismetSystemLibrary.K2_UnPauseTimerHandle` (`self.heatCooldownTimer`)))
          (:`else`))))
    (:`else`)))

(event `AddHeat`
  (bind _tapeheatamount (`self.TapeHeatAmount`))
  ;[1 0 0] Overheated
  (if (< _tapeheatamount (`self.TapeHeatLimit`))
    (set `self.TapeHeatAmount` (+ _tapeheatamount 0.2))
    (`|ExecutionSequence`
      (:`then_0`
        (if (>= _tapeheatamount 80.0)
          (`/Engine/EditorBlueprintResources/StandardMacros.DoOnce` false :!label _label_4
            (:`Completed`
              (`GameplayStatics.PlaySound2D` "/Game/Audio/SND_Tape_OverheatedWarning.SND_Tape_OverheatedWarning" 1.0 1.0 0.0 null null)))
          (else
            (goto _label_4 :!via `Reset`))))
      (:`then_1`
        (if (>= _tapeheatamount 100.0)
          (set `self.TapeHeatAmount` 100.0)
          (`GameplayStatics.PlaySound2D` "/Game/Audio/SND_Tape_Overheated_Cue.SND_Tape_Overheated_Cue" 1.0 1.0 0.0 null null)
          (`WidgetComponent.SetTintColorAndOpacity` (`self.ProgresBarW`) (struct :`R` 1.0 :`A` 1.0))
          (set `self.isOverheated?` true)
          (`self.BeginCoolDownFromHeat`)
          (`FCTweenBPAction.Pause` (`self.TapeProgressTimer`))
          (`self.StopRewindTape`)
          (`KismetSystemLibrary.K2_PauseTimerHandle` (`self.HeatTimer`)))))))

(event `RewindTape`
  (bind _rewindloop (`self.RewindLoop`))
  ;[0 1 0.1351 1 32] Rewind the Tape
  (bind (_asynctaskproxy _value) (`FCTweenBPActionVector.TweenVector` (`self.RewindDefaultLocation`) (- (`SceneComponent.K2_GetComponentLocation` (`self.BP_RewindMachine_Button`)) (0.0 0.0 0.3)) 0.2 "Linear")
    (:`then`
      (`GameplayStatics.PlaySound2D` "/Game/Audio/SND_Tape_Rewind_Pressed_Cue.SND_Tape_Rewind_Pressed_Cue" 1.0 1.0 0.0 null null)
      (if (`self.isOverheated?`)
        (`GameplayStatics.PlaySound2D` "/Game/Audio/SND_Tape_Overheated_Cue.SND_Tape_Overheated_Cue" 1.0 1.0 0.0 null null)
        (else
          (bind _tape (`self.Tape`)
            (:`then`
              (if (`/Game/BLUEPRINTS/Interactables/BP_VHSTape.isRewound?` _tape)
                _
                (elif (< (`/Game/BLUEPRINTS/Interactables/BP_VHSTape.TapeProgress` _tape) 100.0)
                  (`|ExecutionSequence`
                    (:`then_0`
                      (`self.InitProgress`)
                      (`AudioComponent.SetPaused` _rewindloop false)
                      (`AudioComponent.Play` _rewindloop (`self.CurrentRewindLoopPosition`))
                      (bind _returnvalue (`KismetSystemLibrary.K2_SetTimer` null "CheckButtonHover" 0.2 true))
                      (bind _output_get (set `self.ButtonHoverTimer` _returnvalue))
                      (`KismetSystemLibrary.K2_UnPauseTimerHandle` _output_get)
                      (`FCTweenBPAction.Unpause` (`self.TapeProgressTimer`))
                      (bind _asw_press_to_rewind (cast `/Game/BLUEPRINTS/WIDGETS/W_PressToRewind` (`WidgetComponent.GetUserWidgetObject` (`self.PressRewindButtonW`))))
                      (if (> (`Widget.RenderOpacity` (`/Game/BLUEPRINTS/WIDGETS/W_PressToRewind.Border_52` _asw_press_to_rewind)) 0.0)
                        (`/Game/BLUEPRINTS/WIDGETS/W_PressToRewind.RemoveSelf` _asw_press_to_rewind)))
                    (:`then_1`
                      (bind _returnvalue_2 (`KismetSystemLibrary.K2_SetTimer` null "AddHeat" 0.01 true))
                      (bind _output_get_2 (set `self.HeatTimer` _returnvalue_2))
                      (`KismetSystemLibrary.K2_UnPauseTimerHandle` _output_get_2)
                      (`KismetSystemLibrary.K2_PauseTimerHandle` (`self.heatCooldownTimer`)))))))
            (:`else`)))))
    (:`ApplyEasing`
      (`SceneComponent.K2_SetWorldLocation` (`self.BP_RewindMachine_Button`) _value false false))
    (:`OnComplete`
      (`SceneComponent.K2_SetWorldLocation` (`self.CursorDetection`) (`SceneComponent.K2_GetComponentLocation` (`self.BP_RewindMachine_Button`)) false false))))

(event `HeatCooldown`
  (bind _tapeheatamount (`self.TapeHeatAmount`))
  ;[1 0 0] Overheated
  (if (> _tapeheatamount 0.0)
    (set `self.TapeHeatAmount` (- _tapeheatamount 3.0))
    (else
      (set `self.TapeHeatAmount` 0.0))))

(event `BeginCoolDownFromHeat`
  ;[1 0 0] Cooldown after overheat
  (bind (_asynctaskproxy _value) (`FCTweenBPActionFloat.TweenFloat` 100.0 0.0 10.0 "Linear")
    (:`ApplyEasing`
      (set `self.TapeHeatAmount` _value))
    (:`OnComplete`
      (set `self.isOverheated?` false)
      (`WidgetComponent.SetTintColorAndOpacity` (`self.ProgresBarW`) (struct :`R` 1.0 :`G` 1.0 :`B` 1.0 :`A` 1.0)))))

(event `StopRewindTape`
  ;[0 1 0.1351] Release Rewind button
  (bind (_asynctaskproxy _value) (`FCTweenBPActionVector.TweenVector` (`SceneComponent.K2_GetComponentLocation` (`self.BP_RewindMachine_Button`)) (`self.RewindDefaultLocation`) 0.2 "Linear")
    (:`then`
      (`GameplayStatics.PlaySound2D` "/Game/Audio/SND_Tape_Rewind_Released_Cue.SND_Tape_Rewind_Released_Cue" 1.0 1.0 0.0 null null))
    (:`ApplyEasing`
      (`SceneComponent.K2_SetWorldLocation` (`self.BP_RewindMachine_Button`) _value false false))))

(event `/Game/BLUEPRINTS/InteractionBPI.StopInteracting`
  ;[0 1 0.1351] Triggers when mouse leaves rewind button stopped interactring
  (`self.StopRewindTape` :!label _label_5)
  (`KismetSystemLibrary.K2_PauseTimerHandle` (`self.ButtonHoverTimer`))
  (`self.PauseRewind`)
  (bind _tapeprogresstimer (`self.TapeProgressTimer`)
    (:`then`
      (`FCTweenBPAction.Pause` _tapeprogresstimer))
    (:`else`)))

(event `self.CursorDetection.OnComponentEndOverlap`
  (params (OverlappedComponent :type "PrimitiveComponent Object Reference") (OtherActor :type "Actor Object Reference") (OtherComp :type "PrimitiveComponent Object Reference") (OtherBodyIndex :type Integer))
  ;[0 1 0.1351] Triggers when mouse leaves rewind button stopped interactring
  (cast `/Game/BLUEPRINTS/Interactables/BP_RewindMachine_Button` OtherActor)
  (goto _label_5))

(fn `CheckButtonHover`
  (bind (_worldlocation _worlddirection) (`PlayerController.DeprojectMousePositionToWorld` (`GameplayStatics.GetPlayerController` 0)))
  (bind (_outhit _returnvalue) (`KismetSystemLibrary.LineTraceSingle` _worldlocation (+ _worldlocation (* _worlddirection (`self.LTDistance`))) "TraceTypeQuery1"))
  (if _returnvalue
    (`SceneComponent.K2_SetWorldLocation` (`self.CursorDetection`) (`.Location` (`GameplayStatics.BreakHitResult` _outhit)) false false)))

(fn `UserConstructionScript`)