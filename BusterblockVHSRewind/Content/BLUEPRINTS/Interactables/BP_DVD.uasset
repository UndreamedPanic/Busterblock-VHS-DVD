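; BP_DVD is an interactable DVD that can be thrown.
; It records the disc mesh's world location on BeginPlay, and its Throw event applies a stored impulse to that mesh.
; An unfinished SpawnDirt function holds disconnected logic to line-trace from randomly placed points and attach dirt decals to the disc, but none of it runs.
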(event `self.ReceiveBeginPlay`
  (set `self.OGDiscLocation` (`SceneComponent.K2_GetComponentLocation` (`self.SM_DVD`))))

(event `/Game/BLUEPRINTS/Throw_BPI.Throw`
  (`PrimitiveComponent.AddImpulse` (`self.SM_DVD`) (`self.NewImpulse`) "None" false))

(fn `SpawnDirt`)

(fn `UserConstructionScript`)