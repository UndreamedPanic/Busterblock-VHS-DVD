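; Possessable DVD station where the player handles a disc with a rag and spray bottle.
; Possessing it blends the camera in, tweens the tray's current disc into place for rotation, enables boundary walls and adds the UI.
; Looping timers run cursor traces to position the hand target, rag and bottle, while a physics handle grabs interactables.
; Spraying plays effects on a cooldown and briefly pulses the bottle's collision under a "Rag" tag.
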(event `self.ReceiveBeginPlay`
  (`parent.ReceiveBeginPlay`)
  (`PrimitiveComponent.SetCollisionEnabled` (`self.Wall3`) "NoCollision")
  (`PrimitiveComponent.SetCollisionEnabled` (`self.Wall2`) "NoCollision")
  (`PrimitiveComponent.SetCollisionEnabled` (`self.Wall1`) "NoCollision")
  (`PrimitiveComponent.SetCollisionEnabled` (`self.Wall4`) "NoCollision")
  (`EnhancedInputSubsystemInterface.AddMappingContext` (pcsubsystem `EnhancedInputLocalPlayerSubsystem` (`GameplayStatics.GetPlayerController` 0)) "/Game/MODELS/FirstPerson/Input/IMC_Default.IMC_Default" 99 (struct))
  (`self.ToggleRag` false)
  (`self.ToggleBottle` false))

(event `self.ReceivePossessed`
  (params (NewController :type "Controller Object Reference")))

(event `self.ReceiveUnpossessed`
  (params (OldController :type "Controller Object Reference"))
  (`KismetSystemLibrary.K2_PauseTimerHandle` (`self.UpdateHandleTimer`))
  (`PrimitiveComponent.SetCollisionEnabled` (`self.Wall3`) "NoCollision")
  (`PrimitiveComponent.SetCollisionEnabled` (`self.Wall2`) "NoCollision")
  (`PrimitiveComponent.SetCollisionEnabled` (`self.Wall1`) "NoCollision")
  (`PrimitiveComponent.SetCollisionEnabled` (`self.Wall4`) "NoCollision")
  (set `self.isPossessd?` false)
  (`self.ToggleRag` false)
  (`KismetSystemLibrary.K2_PauseTimerHandle` (`self.RagToMouseTimer`))
  (`KismetSystemLibrary.K2_PauseTimerHandle` (`self.BottleToMouseTimer`))
  (bind _dvdui (`self.DVDUI`)
    (:`then`
      (`Widget.RemoveFromParent` _dvdui))
    (:`else`)))

(event `self.ReceiveTick`
  (params (DeltaSeconds :type "Float (single-precision)"))
  (`parent.ReceiveTick` DeltaSeconds))

(event `/Game/BLUEPRINTS/PossessStationBPI.PossessStation`
  (bind _returnvalue (`GameplayStatics.GetPlayerController` 0))
  ;[0 1 0.1351] When possessed
  (`PlayerController.SetViewTargetWithBlend` (`GameplayStatics.GetPlayerController` 0) self 0.5 "VTBlend_EaseInOut" 10.0 true)
  (`KismetSystemLibrary.Delay` 0.5)
  (`Controller.Possess` _returnvalue self)
  (`self.EnableInput` _returnvalue)
  (`self.GrabDiscFromTray`)
  (bind _returnvalue_2 (`KismetSystemLibrary.K2_SetTimer` null "UpdateHandLocation" 0.01 true))
  (set `self.UpdateHandleTimer` _returnvalue_2)
  (`PrimitiveComponent.SetCollisionEnabled` (`self.Wall3`) "QueryAndProbe")
  (`PrimitiveComponent.SetCollisionEnabled` (`self.Wall2`) "QueryAndProbe")
  (`PrimitiveComponent.SetCollisionEnabled` (`self.Wall1`) "QueryAndProbe")
  (`PrimitiveComponent.SetCollisionEnabled` (`self.Wall4`) "QueryAndProbe")
  (set `self.isPossessd?` true)
  (bind _returnvalue_3 (`KismetSystemLibrary.K2_SetTimer` null "AttachRagToMouse" 0.01 true))
  (bind _output_get (set `self.RagToMouseTimer` _returnvalue_3))
  (`KismetSystemLibrary.K2_UnPauseTimerHandle` _output_get)
  (bind _returnvalue_4 (`KismetSystemLibrary.K2_SetTimer` null "AttachBottleToMouse" 0.01 true))
  (bind _output_get_2 (set `self.BottleToMouseTimer` _returnvalue_4))
  (`KismetSystemLibrary.K2_UnPauseTimerHandle` _output_get_2)
  (bind _returnvalue_5 (`|CreateWidget` "/Game/BLUEPRINTS/WIDGETS/W_DVDStation.W_DVDStation_C"))
  (set `self.DVDUI` _returnvalue_5)
  (`UserWidget.AddToViewport` _returnvalue_5 0))

(event `MoveDisc`
  (bind _sm_dvd (`/Game/BLUEPRINTS/Interactables/BP_DVD.SM_DVD` (`self.DVD`)))
  (bind (_asynctaskproxy _value) (`FCTweenBPActionVector.TweenVector` (`SceneComponent.K2_GetComponentLocation` _sm_dvd) (`SceneComponent.K2_GetComponentLocation` (`self.Sphere`)) 0.2 "InOutSine")
    (:`ApplyEasing`
      (`SceneComponent.K2_SetWorldLocation` _sm_dvd _value false false))))

(event `Key|F`
  (params (Key :type "Key Structure"))
  (:`Pressed`
    (if (not (`self.isHoldingObject?`))
      (`self.GrabObject`)
      (bind _returnvalue (`KismetSystemLibrary.K2_SetTimer` null "UpdateTargetLocation" 0.01 true))
      (bind _output_get (set `self.GrabUpdateTimer` _returnvalue))
      (`KismetSystemLibrary.K2_UnPauseTimerHandle` _output_get)
      (else
        (`PhysicsHandleComponent.ReleaseComponent` (`self.PhysicsHandle`) :!label _label)
        (set `self.isHoldingObject?` false)
        (`KismetSystemLibrary.K2_PauseTimerHandle` (`self.GrabUpdateTimer`))))))

(event `GrabDiscFromTray`
  (bind _dvdtray (`self.DVDTray`))
  (bind _output_get (set `self.DVD` (`|GetArrayItem` (`/Game/BLUEPRINTS/BP_DVDTray.DVDsInQueue` _dvdtray) (`/Game/BLUEPRINTS/BP_DVDTray.CurrentDVDID` _dvdtray))))
  (`/Engine/EditorBlueprintResources/StandardMacros.IsValid` _output_get
    (:`Is Valid`
      (bind _sm_dvd (`/Game/BLUEPRINTS/Interactables/BP_DVD.SM_DVD` _output_get))
      (set `/Game/BLUEPRINTS/Interactables/BP_DVD.OGDiscLocation` (`SceneComponent.K2_GetComponentLocation` _sm_dvd) _output_get)
      (`PhysicsHandleComponent.ReleaseComponent` (`/Game/BLUEPRINTS/Interactables/BP_Interactable_Master.PhysicsHandle` _output_get))
      (`PrimitiveComponent.SetSimulatePhysics` _sm_dvd false)
      (`PrimitiveComponent.SetEnableGravity` _sm_dvd false)
      (`self.MoveDisc`))))

(event `EnhancedInput|/Game/MODELS/FirstPerson/Input/Actions/IA_Move`
  (params (ActionValue :type "Vector2D Structure") (ElapsedSeconds :type "Float (double-precision)") (TriggeredSeconds :type "Float (double-precision)") (InputAction :type "InputAction Object Reference" :default "/Game/MODELS/FirstPerson/Input/Actions/IA_Move.IA_Move"))
  (:`Triggered`
    (bind _dvd (`self.DVD`)
      (:`then`
        (bind _sm_dvd (`/Game/BLUEPRINTS/Interactables/BP_DVD.SM_DVD` _dvd))
        (`SceneComponent.K2_AddWorldRotation` _sm_dvd (`KismetMathLibrary.MakeRotator` 0.0 (* (* ActionValue_X -1.0) (`self.RotationSpeed`))) false false)
        (`SceneComponent.K2_AddWorldRotation` _sm_dvd (`KismetMathLibrary.MakeRotator` (* (* ActionValue_Y -1.0) (`self.RotationSpeed`))) false false))
      (:`else`))))

(event `Key|LeftMouseButton`
  (params (Key :type "Key Structure"))
  (:`Pressed`
    (`self.UseSprayBottle`)))

(event `ReleaseObjectFromHand`
  (if (`self.isHoldingObject?`)
    (goto _label)))

(event `Key|Tab`
  (params (Key :type "Key Structure"))
  (:`Pressed`
    (if (`self.isInspectingDisc?`)
      (`PlayerController.SetViewTargetWithBlend` (`GameplayStatics.GetPlayerController` 0) self 0.25 "VTBlend_EaseOut" 1.0 false)
      (set `self.isInspectingDisc?` false)
      (set `self.isHoldingObject?` false)
      (elif (not (`self.isHoldingObject?`))
        (`self.ExitTheStation`)))))

(event `Key|One`
  (params (Key :type "Key Structure"))
  (:`Pressed`
    (`/Engine/EditorBlueprintResources/StandardMacros.FlipFlop`
      (:`A`
        (`self.ToggleRag` true))
      (:`B`
        (`self.ToggleRag` false)))))

(event `Key|Two`
  (params (Key :type "Key Structure"))
  (:`Pressed`
    (`/Engine/EditorBlueprintResources/StandardMacros.FlipFlop`
      (:`A`
        (`self.ToggleBottle` true))
      (:`B`
        (`self.ToggleBottle` false)))))

(event `FlickerBottleTrigger`
  (bind _bottleholder (`self.BottleHolder`))
  (set `ActorComponent.ComponentTags` (`|MakeArray` "Rag" :!type "Name") _bottleholder)
  (`PrimitiveComponent.SetCollisionEnabled` _bottleholder "QueryAndPhysics")
  (`KismetSystemLibrary.Delay` 0.01)
  (`PrimitiveComponent.SetCollisionEnabled` _bottleholder "NoCollision")
  (`KismetArrayLibrary.Array_Clear` (`ActorComponent.ComponentTags` _bottleholder)))

(fn `AttachBottleToMouse`
  (bind (_worldlocation _worlddirection) (`PlayerController.DeprojectMousePositionToWorld` (`GameplayStatics.GetPlayerController` 0)))
  (if (`self.isPossessd?`)
    (bind (_outhit _returnvalue) (`KismetSystemLibrary.LineTraceSingle` _worldlocation (+ _worldlocation (* _worlddirection (`self.LTDistance`))) "TraceTypeQuery1"))
    (if _returnvalue
      (`SceneComponent.K2_SetWorldLocation` (`self.BottleHolder`) (`.Location` (`GameplayStatics.BreakHitResult` _outhit)) false false))))

(fn `AttachRagToMouse`
  (bind (_worldlocation _worlddirection) (`PlayerController.DeprojectMousePositionToWorld` (`GameplayStatics.GetPlayerController` 0)))
  (if (`self.isPossessd?`)
    (bind (_outhit _returnvalue) (`KismetSystemLibrary.LineTraceSingle` _worldlocation (+ _worldlocation (* _worlddirection (`self.LTDistance`))) "TraceTypeQuery1"))
    (if _returnvalue
      (`SceneComponent.K2_SetWorldLocation` (`self.RagHolder`) (`.Location` (`GameplayStatics.BreakHitResult` _outhit)) false false))))

(fn `DetectRagMovement`
  (returns (`hasMoved?` :type Boolean))
  (locals (PreviousMousePosition :type "Vector2D Structure") (CurrentMousePosition :type "Vector2D Structure"))
  (bind (_locationx _locationy) (`PlayerController.GetMousePosition` (`GameplayStatics.GetPlayerController` 0)))
  (`KismetSystemLibrary.PrintString` "Hello")
  (bind _output_get (set `local.PreviousMousePosition` (`KismetMathLibrary.MakeVector2D` _locationx _locationy)))
  (bind _returnvalue (`KismetMathLibrary.NotEqualExactly_Vector2DVector2D` _output_get (`local.CurrentMousePosition`)))
  (`KismetSystemLibrary.PrintString` (`KismetStringLibrary.Conv_BoolToString` _returnvalue))
  (return _returnvalue))

(fn `GrabObject`
  (returns (`isHoldingObject?` :type Boolean))
  (bind _physicshandle (`self.PhysicsHandle`))
  (bind (_worldlocation _worlddirection) (`PlayerController.DeprojectMousePositionToWorld` (`GameplayStatics.GetPlayerController` 0)))
  (bind (_outhit _returnvalue) (`KismetSystemLibrary.LineTraceSingle` _worldlocation (+ _worldlocation (* _worlddirection (`self.LTDistance`))) "TraceTypeQuery1"))
  (if _returnvalue
    (bind (_bblockinghit _binitialoverlap _time _distance _location _impactpoint _normal _impactnormal _physmat _hitactor _hitcomponent) (`GameplayStatics.BreakHitResult` _outhit))
    (bind _asbp_interactable_master (cast `/Game/BLUEPRINTS/Interactables/BP_Interactable_Master` _hitactor))
    (if (`/Game/BLUEPRINTS/Interactables/BP_Interactable_Master.isInteractable?` _asbp_interactable_master)
      (`PhysicsHandleComponent.ReleaseComponent` (`/Game/BLUEPRINTS/Interactables/BP_Interactable_Master.PhysicsHandle` _asbp_interactable_master))
      (if (`KismetSystemLibrary.DoesImplementInterface` _hitactor "/Game/BLUEPRINTS/InteractionBPI.InteractionBPI_C")
        (`PhysicsHandleComponent.GrabComponentAtLocationWithRotation` :`self` _physicshandle :`Component` _hitcomponent :`Location` (`SceneComponent.K2_GetComponentLocation` _hitcomponent))
        (`PhysicsHandleComponent.SetTargetRotation` _physicshandle (`KismetMathLibrary.Conv_VectorToRotator` (`KismetMathLibrary.GetForwardVector` (`SceneComponent.K2_GetComponentRotation` (`self.FirstPersonCamera`)))))
        (set `self.DVD` (cast `/Game/BLUEPRINTS/Interactables/BP_DVD` _hitactor :!pure true))
        (bind _output_get (set `self.isHoldingObject?` true))
        (return _output_get)
        (else
          _)))
    (`self.ReleaseObjectFromHand`)))

(fn `PutDiscInFrontOfScreen`
  (bind (_worldlocation _worlddirection) (`PlayerController.DeprojectMousePositionToWorld` (`GameplayStatics.GetPlayerController` 0)))
  (bind (_outhit _returnvalue) (`KismetSystemLibrary.LineTraceSingle` :`Start` _worldlocation :`End` (+ _worldlocation (* _worlddirection (`self.LTDistance`))) :`TraceChannel` "TraceTypeQuery1" :`DrawDebugType` "Persistent"))
  (if _returnvalue
    (bind _asbp_interactable_master (cast `/Game/BLUEPRINTS/Interactables/BP_Interactable_Master` (`.HitActor` (`GameplayStatics.BreakHitResult` _outhit))))
    (if (`/Game/BLUEPRINTS/Interactables/BP_Interactable_Master.isInteractable?` _asbp_interactable_master)
      (bind _asbp_dvd (cast `/Game/BLUEPRINTS/Interactables/BP_DVD` _asbp_interactable_master))
      (bind _output_get (set `self.DVD` _asbp_dvd))
      (`PrimitiveComponent.SetSimulatePhysics` (`/Game/BLUEPRINTS/Interactables/BP_DVD.SM_DVD` _output_get) false)
      (`PhysicsHandleComponent.ReleaseComponent` (`/Game/BLUEPRINTS/Interactables/BP_Interactable_Master.PhysicsHandle` _output_get))
      (`self.MoveDisc`))))

(fn `SprayBottleCooldown`
  (set `self.canSprayBottle?` true))

(fn `ToggleBottle`
  (params (`On?` :type Boolean))
  (bind _bottleholder (`self.BottleHolder`))
  (bind _bottleholder_2 (`self.BottleHolder`))
  (if `On?`
    (`SceneComponent.SetHiddenInGame` _bottleholder_2 false true)
    (`PrimitiveComponent.SetCollisionEnabled` _bottleholder_2 "QueryAndPhysics")
    (set `self.isBottleEquipped?` true)
    (`self.ToggleRag` false)
    (else
      (`SceneComponent.SetHiddenInGame` _bottleholder true true)
      (`PrimitiveComponent.SetCollisionEnabled` _bottleholder "NoCollision")
      (set `self.isBottleEquipped?` false))))

(fn `ToggleRag`
  (params (`On?` :type Boolean))
  (bind _ragholder (`self.RagHolder`))
  (bind _ragholder_2 (`self.RagHolder`))
  (if `On?`
    (`SceneComponent.SetHiddenInGame` _ragholder_2 false true)
    (`PrimitiveComponent.SetCollisionEnabled` _ragholder_2 "QueryAndPhysics")
    (`self.ToggleBottle` false)
    (else
      (`SceneComponent.SetHiddenInGame` _ragholder true true)
      (`PrimitiveComponent.SetCollisionEnabled` _ragholder "NoCollision"))))

(fn `UpdateHandLocation`
  (bind (_worldlocation _worlddirection) (`PlayerController.DeprojectMousePositionToWorld` (`GameplayStatics.GetPlayerController` 0)))
  (bind (_outhit _returnvalue) (`KismetSystemLibrary.LineTraceSingle` _worldlocation (+ _worldlocation (* _worlddirection (`self.LTDistance`))) "TraceTypeQuery1"))
  (if _returnvalue
    (`SceneComponent.K2_SetWorldLocation` (`self.CursorDetection`) (`KismetMathLibrary.MakeVector` (.x (`.Location` (`GameplayStatics.BreakHitResult` _outhit))) (.y (`.Location` (`GameplayStatics.BreakHitResult` _outhit))) (.z (`SceneComponent.K2_GetComponentLocation` (`self.Hand`)))) false false)))

(fn `UpdateTargetLocation`
  (`PhysicsHandleComponent.SetTargetLocation` (`self.PhysicsHandle`) (`SceneComponent.K2_GetComponentLocation` (`self.CursorDetection`))))

(fn `UserConstructionScript`
  (`parent.UserConstructionScript`))

(fn `UseSprayBottle`
  (if (`self.canSprayBottle?`)
    (if (`self.isBottleEquipped?`)
      (set `self.canSprayBottle?` false)
      (`GameplayStatics.PlaySoundAtLocation` "/Game/Audio/SND_BottleSpray_Cue.SND_BottleSpray_Cue" (`SceneComponent.K2_GetComponentLocation` (`self.SM_SprayBottle`)) (struct) 1.0 1.0 0.0 null null null null)
      (`ActorComponent.SetActive` (`self.NS_SprayBottle`) true true)
      (`KismetSystemLibrary.K2_SetTimer` null "SprayBottleCooldown" 0.55)
      (`self.FlickerBottleTrigger`))))