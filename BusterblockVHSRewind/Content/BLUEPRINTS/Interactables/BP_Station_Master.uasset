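; BP_Station_Master is an interactable station, apparently a base class, that takes player input until Tab exits it.
; Left click line-traces from the mouse cursor and rewinds the RewindMachine's tape on hitting a "Rewind"-tagged component; release calls StopInteracting.
; Exiting calls ExitedStation, blends the view back to BP_FirstPersonCharacter, then repossesses it after a delay and restores its camera rotation.
; It also shows the player HUD again and removes cursor widgets.
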(event `self.ReceiveBeginPlay`
  (bind _returnvalue (`GameplayStatics.GetActorOfClass` "/Game/MODELS/FirstPerson/Blueprints/BP_FirstPersonCharacter.BP_FirstPersonCharacter_C"))
  (set `self.PlayerRef` _returnvalue))

(event `Key|Tab`
  (params (Key :type "Key Structure"))
  (:`Pressed`
    (`self.ExitTheStation`)))

(event `ExitTheStation`
  (bind _returnvalue (`GameplayStatics.GetPlayerController` 0))
  (`|ExecutionSequence`
    (:`then_0`
      (bind _returnvalue_2 (`GameplayStatics.GetActorOfClass` "/Game/MODELS/FirstPerson/Blueprints/BP_FirstPersonCharacter.BP_FirstPersonCharacter_C"))
      (`/Engine/EditorBlueprintResources/StandardMacros.DoOnce` false :!label _label
        (:`Completed`
          (`|ExecutionSequence`
            (:`then_0`
              (`/Game/BLUEPRINTS/PossessStationBPI.ExitedStation`)
              (`PlayerController.SetViewTargetWithBlend` (`GameplayStatics.GetPlayerController` 0) _returnvalue_2 0.5 "VTBlend_EaseInOut" 10.0 false)
              (`KismetSystemLibrary.Delay` 0.5)
              (`Controller.Possess` _returnvalue _returnvalue_2)
              (`self.EnableInput` _returnvalue_2 _returnvalue)
              (`Controller.SetControlRotation` _returnvalue (`/Game/MODELS/FirstPerson/Blueprints/BP_FirstPersonCharacter.LastCameraRotation` _returnvalue_2)))
            (:`then_1`
              (`Widget.SetVisibility` (`/Game/MODELS/FirstPerson/Blueprints/BP_FirstPersonCharacter.PlayerHUDW` _returnvalue_2) "Visible"))
            (:`then_2`
              (bind _foundwidgets (`WidgetBlueprintLibrary.GetAllWidgetsOfClass` "/Game/BLUEPRINTS/WIDGETS/W_Cursor.W_Cursor_C"))
              (for _array_element _foundwidgets
                (`Widget.RemoveFromParent` _array_element)))))))
    (:`then_1`
      (goto _label :!via `Reset`))))

(event `self.ReceiveUnpossessed`
  (params (OldController :type "Controller Object Reference"))
  (goto _label :!via `Reset`))

(event `Key|LeftMouseButton`
  (params (Key :type "Key Structure"))
  (:`Pressed`
    (`self.LinetraceFromView`))
  (:`Released`
    (`/Game/BLUEPRINTS/InteractionBPI.StopInteracting`)))

(fn `LinetraceFromView`
  (bind (_worldlocation _worlddirection) (`PlayerController.DeprojectMousePositionToWorld` (`GameplayStatics.GetPlayerController` 0)))
  (bind (_outhit _returnvalue) (`KismetSystemLibrary.LineTraceSingle` _worldlocation (+ _worldlocation (* _worlddirection (`self.LTDistance`))) "TraceTypeQuery1"))
  (if _returnvalue
    (if (`ActorComponent.ComponentHasTag` (`.HitComponent` (`GameplayStatics.BreakHitResult` _outhit)) "Rewind")
      (bind _rewindmachine (`self.RewindMachine`)
        (:`then`
          (`/Game/BLUEPRINTS/Interactables/BP_RewindMachine.RewindTape` _rewindmachine))
        (:`else`)))))

(fn `UserConstructionScript`)