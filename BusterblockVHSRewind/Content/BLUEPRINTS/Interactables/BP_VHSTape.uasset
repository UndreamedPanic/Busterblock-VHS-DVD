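; Interactable VHS tape that animates its reels to show tape progress and can be thrown.
; BeginPlay hides the left reel and starts a fast looping timer by name on AdjustTapeSize, which also takes Progress and ProgressEnd inputs.
; AdjustTapeSize scales the left tape and right reel oppositely from the progress ratio, reveals the left reel and counter-rotates the spools.
; Throw applies an impulse to the tape mesh.
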(event `self.ReceiveBeginPlay`
  (`KismetSystemLibrary.K2_SetTimer` null "AdjustTapeSize" 0.01 true)
  (`SceneComponent.SetVisibility` (`self.LeftReel`) false true))

(event `AdjustTapeSize`
  (params (Progress :type "Float (double-precision)") (ProgressEnd :type "Float (double-precision)"))
  (bind _returnvalue (* (/ Progress ProgressEnd) -1.0))
  (bind _returnvalue_2 (`KismetMathLibrary.NormalizeToRange` _returnvalue -0.5 -2.0))
  (bind _returnvalue_3 (`KismetMathLibrary.NormalizeToRange` _returnvalue 0.5 2.0))
  (`SceneComponent.SetRelativeScale3D` (`self.SpoolLeftTape`) (`KismetMathLibrary.MakeVector` _returnvalue_3 _returnvalue_3 1.0))
  (`SceneComponent.SetRelativeScale3D` (`self.RightReel`) (`KismetMathLibrary.MakeVector` _returnvalue_2 _returnvalue_2 1.0))
  (`SceneComponent.SetVisibility` (`self.LeftReel`) true true)
  (`SceneComponent.K2_AddWorldRotation` (`self.SpoolRight`) (`KismetMathLibrary.MakeRotator` 0.0 0.0 -8.0) false false)
  (`SceneComponent.K2_AddWorldRotation` (`self.SpoolLeft`) (`KismetMathLibrary.MakeRotator` 0.0 0.0 8.0) false false))

(event `/Game/BLUEPRINTS/Throw_BPI.Throw`
  (`PrimitiveComponent.AddImpulse` (`self.SM_VHSTape`) (`self.NewImpulse`) "None" false))

(fn `UserConstructionScript`)