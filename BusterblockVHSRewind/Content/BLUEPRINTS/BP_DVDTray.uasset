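; BP_DVDTray is a tray actor that tracks which BP_DVD discs sit inside its Box trigger.
; Begin overlap adds the disc to DVDsInQueue with AddUnique and stores the returned index as CurrentDVDID.
; End overlap removes the disc and decrements CurrentDVDID.
; Both paths print the disc count and current ID for debugging.
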(event `self.Box.OnComponentBeginOverlap`
  (params (OverlappedComponent :type "PrimitiveComponent Object Reference") (OtherActor :type "Actor Object Reference") (OtherComp :type "PrimitiveComponent Object Reference") (OtherBodyIndex :type Integer) (bFromSweep :type Boolean) (SweepResult :type "HitResult Structure (by ref)"))
  (bind _asbp_dvd (cast `/Game/BLUEPRINTS/Interactables/BP_DVD` OtherActor))
  (bind _returnvalue (`KismetArrayLibrary.Array_AddUnique` (`self.DVDsInQueue`) _asbp_dvd))
  (set `self.CurrentDVDID` _returnvalue)
  (`KismetSystemLibrary.PrintString` (`KismetStringLibrary.Concat_StrStr` (`KismetStringLibrary.Conv_IntToString` (`KismetArrayLibrary.Array_Length` (`self.DVDsInQueue`))) " Discs" " / " "Current DVD ID " (`KismetStringLibrary.Conv_IntToString` (`self.CurrentDVDID`))) :!label _label))

(event `self.Box.OnComponentEndOverlap`
  (params (OverlappedComponent :type "PrimitiveComponent Object Reference") (OtherActor :type "Actor Object Reference") (OtherComp :type "PrimitiveComponent Object Reference") (OtherBodyIndex :type Integer))
  (bind _dvdsinqueue (`self.DVDsInQueue`))
  (bind _asbp_dvd (cast `/Game/BLUEPRINTS/Interactables/BP_DVD` OtherActor))
  (`KismetArrayLibrary.Array_RemoveItem` _dvdsinqueue (`|GetArrayItem` _dvdsinqueue (`KismetArrayLibrary.Array_Find` _dvdsinqueue _asbp_dvd)))
  (`/Engine/EditorBlueprintResources/StandardMacros.DecrementInt` (`self.CurrentDVDID`)
    (:`  `
      (goto _label))))

(fn `UserConstructionScript`)